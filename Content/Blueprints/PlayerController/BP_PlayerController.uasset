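; Player controller that shows the cursor and lets the mouse rotate or move a clicked BP_RotatableObject_1.
; A left-click cursor trace stores the cast result, which Tick keeps manipulating without checking whether the button is still held.
; Mouse movement rolls the object by default, yaws it with Left Ctrl, or moves it in X/Z with Left Shift.
; Moves apply only within projected screen bounds and print the screen position for debugging.
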(event `Key|LeftMouseButton`
  (params (Key :type "Key Structure"))
  (bind (_deltax _deltay) (`self.GetInputMouseDelta`))
  (bind (_returnvalue_x _returnvalue_y) (`KismetMathLibrary.BreakVector2D` (`WidgetLayoutLibrary.GetViewportSize`)))
  (:`Pressed`
    (bind _asbp_rotatable_object_1 (cast `/Game/Blueprints/Actors/Interactables/BP_RotatableObject_1` (`.HitActor` (`GameplayStatics.BreakHitResult` (`self.GetHitResultUnderCursorByChannel` "TraceTypeQuery2")))))
    (`/Engine/EditorBlueprintResources/StandardMacros.IsValid` _asbp_rotatable_object_1 :!label _label
      (:`Is Valid`
        (if (`self.IsInputKeyDown` "LeftControl")
          (`self.K2_AddActorWorldRotation` _asbp_rotatable_object_1 (`KismetMathLibrary.MakeRotator` 0.0 0.0 (* _deltax 10.0)) false false)
          (elif (`self.IsInputKeyDown` "LeftShift")
            (bind (_returnvalue_x_2 _returnvalue_y_2 _returnvalue_z) (`KismetMathLibrary.BreakVector` (`self.K2_GetActorLocation` _asbp_rotatable_object_1)))
            (bind _returnvalue (- _returnvalue_x_2 _deltax))
            (bind _returnvalue_2 (+ _deltay _returnvalue_z))
            (bind _screenlocation (`self.ProjectWorldLocationToScreen` (`KismetMathLibrary.MakeVector` _returnvalue _returnvalue_y_2 _returnvalue_2)))
            (if (> (`KismetMathLibrary.BreakVector2D` _screenlocation) 80.0)
              (if (> (`.Y` (`KismetMathLibrary.BreakVector2D` _screenlocation)) 80.0)
                (if (< (`.Y` (`KismetMathLibrary.BreakVector2D` _screenlocation)) _returnvalue_y)
                  (if (< (`KismetMathLibrary.BreakVector2D` _screenlocation) _returnvalue_x)
                    (`self.K2_SetActorLocation` _asbp_rotatable_object_1 (`KismetMathLibrary.MakeVector` _returnvalue _returnvalue_y_2 _returnvalue_2) false false)
                    (bind _screenlocation_2 (`self.ProjectWorldLocationToScreen` (`self.K2_GetActorLocation` _asbp_rotatable_object_1)))
                    (`KismetSystemLibrary.PrintString` (`KismetStringLibrary.Conv_Vector2dToString` (`KismetMathLibrary.MakeVector2D` (`KismetMathLibrary.BreakVector2D` _screenlocation_2) (`.Y` (`KismetMathLibrary.BreakVector2D` _screenlocation_2)))))))))
            (else
              (`self.K2_AddActorWorldRotation` _asbp_rotatable_object_1 (`KismetMathLibrary.MakeRotator` (* _deltay -10.0)) false false))))))))

(event `self.ReceiveTick`
  (params (DeltaSeconds :type "Float (single-precision)"))
  (goto _label))

(event `self.ReceiveBeginPlay`
  (set `self.bShowMouseCursor` true))

(fn `UserConstructionScript`)