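; BP_RotatableObject is an interactable actor that the player rotates by holding an input and moving the mouse.
; The RotateObjectHorizontaly action toggles an IsRotating flag, and while it is set Tick applies inverted, scaled mouse Y delta to the actor's pitch, despite the action's name.
; Cursor hover only prints a debug message and does not gate rotation; the MouseX and MouseY events are empty.
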(event `InputAction|RotateObjectHorizontaly`
  (params (Key :type "Key Structure"))
  (:`Pressed`
    (`KismetSystemLibrary.PrintString` "CLICKED \n")
    (set `self.IsRotating` true))
  (:`Released`
    (`KismetSystemLibrary.PrintString` "RELEASED")
    (set `self.IsRotating` false)))

(event `self.ReceiveTick`
  (params (DeltaSeconds :type "Float (single-precision)"))
  (if (`self.IsRotating`)
    (`self.K2_SetActorRotation` (`KismetMathLibrary.MakeRotator` (.roll (`self.K2_GetActorRotation`)) (+ (.pitch (`self.K2_GetActorRotation`)) (* (`.DeltaY` (`PlayerController.GetInputMouseDelta` (`GameplayStatics.GetPlayerController` 0))) -10.0)) (.yaw (`self.K2_GetActorRotation`))))))

(event `self.ReceiveActorBeginCursorOver`
  (`KismetSystemLibrary.PrintString` "Hello"))

(event `InputAxisKey|MouseX`
  (params (AxisValue :type "Float (single-precision)")))

(event `InputAxisKey|MouseY`
  (params (AxisValue :type "Float (single-precision)")))

(fn `UserConstructionScript`)